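; Base weapon Blueprint that sets its displayed mesh from a publicly chosen weapon class and index.
; The Construction Script switches on the WeaponClass enum, takes the keys of that class's map and applies the one at WeaponNum to the Weapon static mesh.
; None clears the mesh.
; Rocket Launcher reads SRWeapon and Sniper Rifle reads RLWeapon, so those map names appear swapped.
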(fn `UserConstructionScript`
  ;[0 0 0] Weapon Classes with using Map and Enums to set specific Weapons publicly
  (switch `/Game/Blueprints/Data/Enum/WeaponType_Enum` (`self.Weapon Class`)
    (:`NewEnumerator7`
      (`StaticMeshComponent.SetStaticMesh` (`self.Weapon`) null))
    (:`NewEnumerator0`
      (bind _keys (`BlueprintMapLibrary.Map_Keys` (`self.Melee Weapon`)))
      (`StaticMeshComponent.SetStaticMesh` (`self.Weapon`) (`|GetArrayItem` _keys (`self.WeaponNum`))))
    (:`NewEnumerator1`
      (bind _keys_2 (`BlueprintMapLibrary.Map_Keys` (`self.Pistol Weapon`)))
      (`StaticMeshComponent.SetStaticMesh` (`self.Weapon`) (`|GetArrayItem` _keys_2 (`self.WeaponNum`))))
    (:`NewEnumerator2`
      (bind _keys_3 (`BlueprintMapLibrary.Map_Keys` (`self.SMG Weapon`)))
      (`StaticMeshComponent.SetStaticMesh` (`self.Weapon`) (`|GetArrayItem` _keys_3 (`self.WeaponNum`))))
    (:`NewEnumerator5`
      (bind _keys_4 (`BlueprintMapLibrary.Map_Keys` (`self.AR Weapon`)))
      (`StaticMeshComponent.SetStaticMesh` (`self.Weapon`) (`|GetArrayItem` _keys_4 (`self.WeaponNum`))))
    (:`NewEnumerator4`
      (bind _keys_5 (`BlueprintMapLibrary.Map_Keys` (`self.Shotgun Weapon`)))
      (`StaticMeshComponent.SetStaticMesh` (`self.Weapon`) (`|GetArrayItem` _keys_5 (`self.WeaponNum`))))
    (:`NewEnumerator3`
      (bind _keys_6 (`BlueprintMapLibrary.Map_Keys` (`self.SR Weapon`)))
      (`StaticMeshComponent.SetStaticMesh` (`self.Weapon`) (`|GetArrayItem` _keys_6 (`self.WeaponNum`))))
    (:`NewEnumerator8`
      (bind _keys_7 (`BlueprintMapLibrary.Map_Keys` (`self.RL Weapon`)))
      (`StaticMeshComponent.SetStaticMesh` (`self.Weapon`) (`|GetArrayItem` _keys_7 (`self.WeaponNum`))))))