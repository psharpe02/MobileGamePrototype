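; Timed explosive projectile actor that detonates on a timer started at BeginPlay, with no impact logic in its graph.
; Detonation removes the projectile component, spawns a particle effect, fires a radial impulse and applies radial damage, with debug text and sphere.
; It also schedules a delayed sound and reports a noise event for AI hearing.
; The spawned emitter is destroyed immediately, and the actor one second later.
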(event `self.ReceiveBeginPlay`
  ;[0.1667 1 0] Event Timer to spawn projectile emitter
  (`KismetSystemLibrary.K2_SetTimerDelegate` (delegate `Detonate`) (`self.Projectile Detonate`)))

(event `Detonate`
  ;[0.1667 1 0] Event Timer to spawn projectile emitter
  (`ActorComponent.K2_DestroyComponent` (`self.Projectile`))
  (`KismetSystemLibrary.PrintString` "Projectile Destroyed" true true (struct :`R` 1.0 :`A` 1.0) 5.0)
  (bind _returnvalue (`GameplayStatics.SpawnEmitterAtLocation` (`self.Particle System`) (`self.K2_GetActorLocation`)))
  ;[1 0 0] Debugging and Applying Impulse and Radial Damage
  (`RadialForceComponent.FireImpulse` (`self.RadialForce`))
  (`GameplayStatics.ApplyRadialDamage` :`BaseDamage` (`self.Base Damage`) :`Origin` (`self.K2_GetActorLocation`) :`DamageRadius` (`self.Damage Radius`) :`DamageCauser` null :`InstigatedByController` null)
  (`KismetSystemLibrary.DrawDebugSphere` (`self.K2_GetActorLocation`) (`self.Damage Radius`))
  ;[0 0.3167 1] Play Sound Effect
  (`KismetSystemLibrary.K2_SetTimerDelegate` (delegate `Play Sound Effect`) (`self.Sound Timer`))
  (`AISense_Hearing.ReportNoiseEvent` (`self.K2_GetActorLocation`) 1.0 self 1200.0)
  ;[1 0 0] Destroy Nodes
  (`ActorComponent.K2_DestroyComponent` _returnvalue)
  (`KismetSystemLibrary.Delay` 1.0)
  (`self.K2_DestroyActor`))

(event `Play Sound Effect`
  ;[0 0.3167 1] Play Sound Effect
  (`GameplayStatics.PlaySoundAtLocation` (`self.Sound Effect`) (`self.K2_GetActorLocation`) (struct) 1.0 1.0 0.0 null null null null))

(fn `UserConstructionScript`)