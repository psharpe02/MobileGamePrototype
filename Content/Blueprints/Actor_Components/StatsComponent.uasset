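; Actor component that tracks health, stamina and infection for its owner, in what appears to be a turn-based game.
; Events adjust and print stats, mostly clamped, and Tick uses a DoOnce to grant stamina once per StaminaTurn.
; ActorDeath, not called within this graph, destroys the owner with sound and particles at zero health or full infection.
; CheckStats sets UseItem in sequence, so only the final Infection check determines the result.
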(event `self.ReceiveTick`
  (params (DeltaSeconds :type "Float (single-precision)"))
  (`|ExecutionSequence`
    (:`then_0`
      ;[0 0 0] Add Stamina to owner each turn
      (if (`self.Stamina Turn?`)
        (`/Engine/EditorBlueprintResources/StandardMacros.DoOnce` false :!label _label
          (:`Completed`
            (`self.Add Stamina` 50)))
        (else
          (goto _label :!via `Reset`))))))

(event `self.ReceiveBeginPlay`
  ;[0 0 0] Event Begin Play
  (set `self.Health` (`self.Max Health`))
  (set `self.Stamina` (`self.Max Stamina`))
  (set `self.Infection` (`self.Infection`))
  (set `self.Death` (`self.Death`))
  (set `self.Owner` (`self.GetOwner`)))

(event `Actor Death`
  (bind _returnvalue (`Actor.K2_GetActorLocation` (`self.Owner`)))
  ;[0 0 0] Character Stats
  ;;[0 0 0] Actor's Death
  (if (or (<= (`self.Health`) 0) (>= (`self.Infection`) 100))
    (`GameplayStatics.PlaySoundAtLocation` (`self.Sound`) _returnvalue (struct) 1.0 1.0 0.0 null null null null)
    (`GameplayStatics.SpawnEmitterAtLocation` (`self.Emitter Template`) _returnvalue)
    (set `self.Death` true)
    (`Actor.K2_DestroyActor` (`self.Owner`))))

(event `Add Health`
  (params (`Add Health` :type Integer))
  ;[0 0 0] Character Stats
  ;;[0 0 0] Add Health
  (set `self.Health` (`KismetMathLibrary.Clamp` (+ `Add Health` (`self.Health`)) 0 100)))

(event `Add Stamina`
  (params (Stamina :type Integer))
  ;[0 0 0] Character Stats
  ;;[0 0 0] Add Stamina
  (bind _output_get (set `self.Stamina` (`KismetMathLibrary.Clamp` (+ Stamina (`self.Stamina`)) 0 100)))
  ;;[0 0 0] Checks Stamina Value if it is under or over the limit
  (if (>= _output_get 100)
    (`KismetSystemLibrary.PrintString` "Stamina is full")
    (else
      (`KismetSystemLibrary.PrintString` (`KismetStringLibrary.Conv_IntToString` (`self.Stamina`)) :!label _label_2))))

(event `Take Damage`
  (params (Damage :type Integer))
  ;[0 0 0] Character Stats
  ;;[0 0 0] Take Damage
  (bind _output_get (set `self.Health` (- (`self.Health`) Damage)))
  (`KismetSystemLibrary.PrintString` (`KismetStringLibrary.Conv_IntToString` _output_get)))

(event `Remove Stamina`
  (params (Stamina :type Integer))
  ;[0 0 0] Character Stats
  ;;[0 0 0] Remove Stamina
  (bind _output_get (set `self.Stamina` (`KismetMathLibrary.Clamp` (- (`self.Stamina`) Stamina) 0 100)))
  ;;[0 0 0] Checks Stamina Value if it is under or over the limit
  (if (<= _output_get 0)
    (`KismetSystemLibrary.PrintString` "No More Stamina ")
    (else
      (goto _label_2))))

(event `Add Infection`
  (params (`Infection Value` :type Integer))
  ;[0 0 0] Character Stats
  ;;[0 0 0] Actor More Infected
  (bind _output_get (set `self.Infection` (`KismetMathLibrary.Clamp` (+ (`self.Infection`) `Infection Value`) 0 100)))
  (`KismetSystemLibrary.PrintString` (`KismetStringLibrary.Conv_IntToString` _output_get)))

(event `Remove Infection`
  (params (`Infection Value` :type Integer))
  ;[0 0 0] Character Stats
  ;;[0 0 0] Actor Less Infected
  (bind _output_get (set `self.Infection` (`KismetMathLibrary.Clamp` (- (`self.Infection`) `Infection Value`) 0 100)))
  (`KismetSystemLibrary.PrintString` (`KismetStringLibrary.Conv_IntToString` _output_get)))

(fn `CheckStats`
  (`|ExecutionSequence`
    (:`then_0`
      (if (== (`self.Health`) (`self.Max Health`))
        (set `self.Use Item?` false)
        (else
          (set `self.Use Item?` true))))
    (:`then_1`
      (if (== (`self.Stamina`) (`self.Max Stamina`))
        (set `self.Use Item?` false)
        (else
          (set `self.Use Item?` true))))
    (:`then_2`
      (if (== (`self.Infection`) 0)
        (set `self.Use Item?` false)
        (else
          (set `self.Use Item?` true))))))