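; Character component that dresses a player or zombie character with modular head, body, glasses and backpack skeletal meshes.
; SetCharacterMesh stores the four mesh components, then picks meshes from per-type arrays via nested selects on character type, gender, enemy type and part indices.
; It applies the meshes and sets a white or black skin material on head and body.
; Only male civilian, worker and law zombies are wired among enemies.
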(event `self.ReceiveBeginPlay`
  ;[0 0 0] Event Begin Play
  (set `self.Owner` (`self.GetOwner`)))

(event `Set Character Mesh`
  (params (Head :type "SkeletalMeshComponent Object Reference") (Body :type "SkeletalMeshComponent Object Reference") (Glasses :type "SkeletalMeshComponent Object Reference") (Backpack :type "SkeletalMeshComponent Object Reference"))
  (bind (_male_character_head _male_character_body _male_character_glasses _male_character_backpack) (break `/Game/Blueprints/Data/Struct/ActorInfo/Male_Character` (`self.Male Character`)))
  (bind (_female_character_head _female_character_body _female_character_glasses _female_character_backpack) (break `/Game/Blueprints/Data/Struct/ActorInfo/Female_Character` (`self.Female Character`)))
  (bind _gender_type (`self.Gender Type`))
  (bind (_custom_character_head _custom_character_body _custom_character_glasses _custom_character_backpack) (break `/Game/Blueprints/Data/Struct/ActorInfo/Female_Character` (`self.Custom Character`)))
  (bind (_m_zombie_civilian_head _m_zombie_civilian_body _m_zombie_civilian_glasses _m_zombie_civilian_backpack) (break `/Game/Blueprints/Data/Struct/EnemyInfo/M_Zombie_Civilian` (`self.M_Zombie_Civilian`)))
  (bind (_m_zombie_law_head _m_zombie_law_body _m_zombie_law_glasses _m_zombie_law_backpack) (break `/Game/Blueprints/Data/Struct/EnemyInfo/M_Zombie_Law` (`self.M_Zombie_Law`)))
  (bind (_m_zombie_worker_head _m_zombie_worker_body _m_zombie_worker_glasses _m_zombie_worker_backpack) (break `/Game/Blueprints/Data/Struct/EnemyInfo/M_Zombie_Worker` (`self.M_Zombie_Worker`)))
  ;[0 0 0] Gets current Character skeletal meshes that from male and female structures
  (set `self.Head` Head)
  (set `self.Body` Body)
  (set `self.Glasses` Glasses)
  (set `self.Backpack` Backpack)
  ;[0 0 0] Sets Character skeletal meshes and name
  (bind _output_get (set `self.Current Character` (make `/Game/Blueprints/Data/Struct/ActorInfo/Current_Character` (`self.Name`) (select `/Game/Blueprints/Data/Enum/Character/Character_Type` (`self.Character Type`) :`NewEnumerator0` (`|GetArrayItem` (select `/Game/Blueprints/Data/Enum/Character/Gender_Enum` _gender_type :`NewEnumerator0` _male_character_head :`NewEnumerator1` _female_character_head :`NewEnumerator3` _custom_character_head) (`self.Head Num`)) :`NewEnumerator1` (select `/Game/Blueprints/Data/Enum/Character/Enemy_Type` (`self.Enemy Type`) :`NewEnumerator6` (`|GetArrayItem` (select `/Game/Blueprints/Data/Enum/Character/Gender_Enum` (`self.Gender Type`) :`NewEnumerator0` _m_zombie_civilian_head) (`self.Full Body`)) :`NewEnumerator8` (`|GetArrayItem` (select `/Game/Blueprints/Data/Enum/Character/Gender_Enum` (`self.Gender Type`) :`NewEnumerator0` _m_zombie_worker_head) (`self.Full Body`)) :`NewEnumerator9` (`|GetArrayItem` (select `/Game/Blueprints/Data/Enum/Character/Gender_Enum` (`self.Gender Type`) :`NewEnumerator0` _m_zombie_law_head) (`self.Full Body`)))) (select `/Game/Blueprints/Data/Enum/Character/Character_Type` (`self.Character Type`) :`NewEnumerator0` (`|GetArrayItem` (select `/Game/Blueprints/Data/Enum/Character/Gender_Enum` _gender_type :`NewEnumerator0` _male_character_body :`NewEnumerator1` _female_character_body :`NewEnumerator3` _custom_character_body) (`self.Body Num`)) :`NewEnumerator1` (select `/Game/Blueprints/Data/Enum/Character/Enemy_Type` (`self.Enemy Type`) :`NewEnumerator6` (`|GetArrayItem` (select `/Game/Blueprints/Data/Enum/Character/Gender_Enum` (`self.Gender Type`) :`NewEnumerator0` _m_zombie_civilian_body) (`self.Full Body`)) :`NewEnumerator8` (`|GetArrayItem` (select `/Game/Blueprints/Data/Enum/Character/Gender_Enum` (`self.Gender Type`) :`NewEnumerator0` _m_zombie_worker_body) (`self.Glasses Num`)) :`NewEnumerator9` (`|GetArrayItem` (select `/Game/Blueprints/Data/Enum/Character/Gender_Enum` (`self.Gender Type`) :`NewEnumerator0` _m_zombie_law_body) (`self.Glasses Num`)))) (select `/Game/Blueprints/Data/Enum/Character/Character_Type` (`self.Character Type`) :`NewEnumerator0` (`|GetArrayItem` (select `/Game/Blueprints/Data/Enum/Character/Gender_Enum` _gender_type :`NewEnumerator0` _male_character_glasses :`NewEnumerator1` _female_character_glasses :`NewEnumerator3` _custom_character_glasses) (`self.Glasses Num`)) :`NewEnumerator1` (select `/Game/Blueprints/Data/Enum/Character/Enemy_Type` (`self.Enemy Type`) :`NewEnumerator6` (`|GetArrayItem` (select `/Game/Blueprints/Data/Enum/Character/Gender_Enum` (`self.Gender Type`) :`NewEnumerator0` _m_zombie_civilian_glasses) (`self.Glasses Num`)) :`NewEnumerator8` (`|GetArrayItem` (select `/Game/Blueprints/Data/Enum/Character/Gender_Enum` (`self.Gender Type`) :`NewEnumerator0` _m_zombie_worker_glasses) (`self.Glasses Num`)) :`NewEnumerator9` (`|GetArrayItem` (select `/Game/Blueprints/Data/Enum/Character/Gender_Enum` (`self.Gender Type`) :`NewEnumerator0` _m_zombie_law_glasses) (`self.Glasses Num`)))) (select `/Game/Blueprints/Data/Enum/Character/Character_Type` (`self.Character Type`) :`NewEnumerator0` (`|GetArrayItem` (select `/Game/Blueprints/Data/Enum/Character/Gender_Enum` _gender_type :`NewEnumerator0` _male_character_backpack :`NewEnumerator1` _female_character_backpack :`NewEnumerator3` _custom_character_backpack) (`self.Backpack Num`)) :`NewEnumerator1` (select `/Game/Blueprints/Data/Enum/Character/Enemy_Type` (`self.Enemy Type`) :`NewEnumerator6` (`|GetArrayItem` (select `/Game/Blueprints/Data/Enum/Character/Gender_Enum` (`self.Gender Type`) :`NewEnumerator0` _m_zombie_civilian_backpack) (`self.Backpack Num`)) :`NewEnumerator8` (`|GetArrayItem` (select `/Game/Blueprints/Data/Enum/Character/Gender_Enum` (`self.Gender Type`) :`NewEnumerator0` _m_zombie_worker_backpack) (`self.Backpack Num`)) :`NewEnumerator9` (`|GetArrayItem` (select `/Game/Blueprints/Data/Enum/Character/Gender_Enum` (`self.Gender Type`) :`NewEnumerator0` _m_zombie_law_backpack) (`self.Backpack Num`)))))))
  (`|ExecutionSequence`
    (:`then_0`
      (bind ((`Head_103_BE8AEA0D491232E80D98098EA613B953` _head) (`Body_104_523184E94E96F3BE88B24D9C37E1FE01` _body) (`Glasses_105_0B3B6A7F474503C6F5F3B1B63CC78ADA` _glasses) (`Backpack_106_934F3DB7401917F6EB916D96AFF6B0CC` _backpack)) (break `/Game/Blueprints/Data/Struct/ActorInfo/Current_Character` _output_get))
      (`SkinnedMeshComponent.SetSkinnedAssetAndUpdate` (`self.Head`) _head true)
      (`SkinnedMeshComponent.SetSkinnedAssetAndUpdate` (`self.Body`) _body true)
      (`SkinnedMeshComponent.SetSkinnedAssetAndUpdate` (`self.Glasses`) _glasses true)
      (`SkinnedMeshComponent.SetSkinnedAssetAndUpdate` (`self.Backpack`) _backpack true))
    (:`then_1`
      (switch `/Game/Blueprints/Data/Enum/Character/Skin_Enum` (`self.Skin Type`)
        (:`NewEnumerator0`
          (`PrimitiveComponent.SetMaterial` (`self.Head`) 0 "/Game/TopDown/Player/Materials/M_Citizens_A.M_Citizens_A")
          (`PrimitiveComponent.SetMaterial` (`self.Body`) 0 "/Game/TopDown/Player/Materials/M_Citizens_A.M_Citizens_A"))
        (:`NewEnumerator1`
          (`PrimitiveComponent.SetMaterial` (`self.Body`) 0 "/Game/TopDown/Player/Materials/M_Citizens_B.M_Citizens_B")
          (`PrimitiveComponent.SetMaterial` (`self.Head`) 0 "/Game/TopDown/Player/Materials/M_Citizens_B.M_Citizens_B"))))))