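; Actor component that tracks a stamina value for its owning actor.
; On BeginPlay it fills stamina to MaxStamina and caches the owner.
; Add and Remove events change the value, clamped to a hard-coded integer range of 0 to 100 independent of MaxStamina.
; Each change prints the current value, or a message when stamina is full or empty.
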(event `self.ReceiveBeginPlay`
  ;[0 0 0] Event Begin Play
  (set `self.Stamina` (`self.Max Stamina`))
  (set `self.Owner` (`self.GetOwner`)))

(event `Add Stamina`
  (params (Stamina :type Integer))
  ;[0 0 0] Add Stamina
  (bind _output_get (set `self.Stamina` (`KismetMathLibrary.Clamp` (+ Stamina (`self.Stamina`)) 0 100)))
  ;[0 0 0] Checks Stamina Value if it is under or over the limit
  (if (>= _output_get 100)
    (`KismetSystemLibrary.PrintString` "Stamina is full")
    (else
      (`KismetSystemLibrary.PrintString` (`KismetStringLibrary.Conv_IntToString` (`self.Stamina`)) :!label _label))))

(event `Remove Stamina`
  (params (Stamina :type Integer))
  ;[0 0 0] Remove Stamina
  (bind _output_get (set `self.Stamina` (`KismetMathLibrary.Clamp` (- (`self.Stamina`) Stamina) 0 100)))
  ;[0 0 0] Checks Stamina Value if it is under or over the limit
  (if (<= _output_get 0)
    (`KismetSystemLibrary.PrintString` "No More Stamina ")
    (else
      (goto _label))))