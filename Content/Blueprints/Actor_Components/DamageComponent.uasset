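; DamageComponent is an actor component that subtracts a damage amount from the health of the actor that owns it.
; BeginPlay caches the owner and sets Damage to itself.
; TakeDamage finds the owner's HealthComponent, lowers its Health by the stored Damage if the component is valid, and prints the new value.
; Health is written directly, with no clamping or death handling here.
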(event `self.ReceiveBeginPlay`
  ;[0 0 0] Event Begin Play
  (set `self.Damage` (`self.Damage`))
  (set `self.Owner` (`self.GetOwner`)))

(event `Take Damage`
  (bind _returnvalue (`Actor.GetComponentByClass` (`self.Owner`) "/Game/Blueprints/Actor_Components/HealthComponent.HealthComponent_C"))
  ;[0 0 0] Take Damage
  (`/Engine/EditorBlueprintResources/StandardMacros.IsValid` _returnvalue
    (:`Is Valid`
      (bind _output_get (set `/Game/Blueprints/Actor_Components/HealthComponent.Health` (- (`/Game/Blueprints/Actor_Components/HealthComponent.Health` _returnvalue) (`self.Damage`)) _returnvalue))
      (`KismetSystemLibrary.PrintString` (`KismetStringLibrary.Conv_IntToString` _output_get)))))