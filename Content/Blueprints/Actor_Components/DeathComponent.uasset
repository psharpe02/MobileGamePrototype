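; Actor component that handles the death of its owning actor, caching the owner at Begin Play.
; When ActorDeath is called, it checks the owner's HealthComponent for depleted health, then its InfectionComponent for full infection.
; Either condition plays a sound, spawns an emitter, sets the Death flag and destroys the owner.
; The infection check only runs when a valid HealthComponent exists.
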(event `self.ReceiveBeginPlay`
  ;[0 0 0] Event Begin Play
  (set `self.Death` (`self.Death`))
  (set `self.Owner` (`self.GetOwner`)))

(event `Actor Death`
  (bind _owner (`self.Owner`))
  (bind _returnvalue (`Actor.GetComponentByClass` _owner "/Game/Blueprints/Actor_Components/InfectionComponent.InfectionComponent_C"))
  (bind _returnvalue_2 (`Actor.GetComponentByClass` _owner "/Game/Blueprints/Actor_Components/HealthComponent.HealthComponent_C"))
  (bind _returnvalue_3 (`Actor.K2_GetActorLocation` (`self.Owner`)))
  ;[0 0 0] Actor's Death
  (`/Engine/EditorBlueprintResources/StandardMacros.IsValid` _returnvalue_2
    (:`Is Valid`
      (if (<= (`/Game/Blueprints/Actor_Components/HealthComponent.Health` _returnvalue_2) 0)
        (`GameplayStatics.PlaySoundAtLocation` (`self.Sound`) _returnvalue_3 (struct) 1.0 1.0 0.0 null null null null :!label _label)
        (`GameplayStatics.SpawnEmitterAtLocation` (`self.Emitter Template`) _returnvalue_3)
        (set `self.Death` true)
        (`Actor.K2_DestroyActor` (`self.Owner`))
        (else
          (`/Engine/EditorBlueprintResources/StandardMacros.IsValid` _returnvalue
            (:`Is Valid`
              (if (>= (`/Game/Blueprints/Actor_Components/InfectionComponent.Infection` _returnvalue) 100)
                (goto _label)
                (else
                  _)))
            (:`Is Not Valid`
              _))
          (`KismetSystemLibrary.PrintString` "Actor Not Dead"))))))