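; Actor component that manages the equipped item across health, stamina, infection, explosive, heat and distract categories.
; SelectItem applies the mesh and transform for ItemClass and ItemNum from per-category maps keyed by static mesh.
; SetCurrentItem stores that mesh in its category's CurrentItems slot.
; SwapCurrentItem falls through to the next filled slot, recovering class, index and transform by mesh lookup, or to None when slot zero is empty.
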(event `self.ReceiveBeginPlay`
  ;[0 0 0] Event Begin Play
  (set `self.Owner` (`self.GetOwner`)))

(event `Select Item`
  (params (Item :type "StaticMeshComponent Object Reference"))
  (bind _item_num (`self.Item Num`))
  (bind _stamina_item (`self.Stamina Item`))
  (bind _item_num_2 (`self.Item Num`))
  (bind _infection_item (`self.Infection Item`))
  (bind _item_num_3 (`self.Item Num`))
  (bind _health_item (`self.Health Item`))
  (bind _item_num_4 (`self.Item Num`))
  (bind _heat_item (`self.Heat Item`))
  (bind _distract_item (`self.Distract Item`))
  (bind _item_num_5 (`self.Item Num`))
  (bind _explosive_item (`self.Explosive Item`))
  (bind _item_num_6 (`self.Item Num`))
  ;[0 0 0] Select Item From Item Classes
  (set `self.Item` Item)
  (switch `/Game/Blueprints/Data/Enum/ItemTypes/ItemType_Enum` (`self.Item Class`)
    (:`NewEnumerator7`
      (`StaticMeshComponent.SetStaticMesh` (`self.Item`) null))
    (:`NewEnumerator11`
      (bind _keys (`BlueprintMapLibrary.Map_Keys` _health_item))
      (bind _values (`BlueprintMapLibrary.Map_Values` _health_item))
      (`StaticMeshComponent.SetStaticMesh` (`self.Item`) (`|GetArrayItem` _keys _item_num))
      (`SceneComponent.K2_SetRelativeTransform` (`self.Item`) (`.Transform_122_52165CD641C2D4A94A776894C4A9C928` (break `/Game/Blueprints/Data/Struct/ItemInfo/Health_Item_Info` (`|GetArrayItem` _values _item_num))) false false))
    (:`NewEnumerator12`
      (bind _keys_2 (`BlueprintMapLibrary.Map_Keys` _stamina_item))
      (bind _values_2 (`BlueprintMapLibrary.Map_Values` _stamina_item))
      (`StaticMeshComponent.SetStaticMesh` (`self.Item`) (`|GetArrayItem` _keys_2 _item_num_6))
      (`SceneComponent.K2_SetRelativeTransform` (`self.Item`) (`.Transform_122_52165CD641C2D4A94A776894C4A9C928` (break `/Game/Blueprints/Data/Struct/ItemInfo/Stamina_Item_Info` (`|GetArrayItem` _values_2 _item_num_6))) false false))
    (:`NewEnumerator14`
      (bind _keys_3 (`BlueprintMapLibrary.Map_Keys` _infection_item))
      (bind _values_3 (`BlueprintMapLibrary.Map_Values` _infection_item))
      (`StaticMeshComponent.SetStaticMesh` (`self.Item`) (`|GetArrayItem` _keys_3 _item_num_2))
      (`SceneComponent.K2_SetRelativeTransform` (`self.Item`) (`.Transform_122_52165CD641C2D4A94A776894C4A9C928` (break `/Game/Blueprints/Data/Struct/ItemInfo/Infection_Item_Info` (`|GetArrayItem` _values_3 _item_num_2))) false false))
    (:`NewEnumerator0`
      (bind _keys_4 (`BlueprintMapLibrary.Map_Keys` _explosive_item))
      (bind _values_4 (`BlueprintMapLibrary.Map_Values` _explosive_item))
      (`StaticMeshComponent.SetStaticMesh` (`self.Item`) (`|GetArrayItem` _keys_4 _item_num_5))
      (`SceneComponent.K2_SetRelativeTransform` (`self.Item`) (`.Transform_122_52165CD641C2D4A94A776894C4A9C928` (break `/Game/Blueprints/Data/Struct/ItemInfo/Explosive_Item_Info` (`|GetArrayItem` _values_4 _item_num_5))) false false))
    (:`NewEnumerator15`
      (bind _keys_5 (`BlueprintMapLibrary.Map_Keys` _heat_item))
      (bind _values_5 (`BlueprintMapLibrary.Map_Values` _heat_item))
      (`StaticMeshComponent.SetStaticMesh` (`self.Item`) (`|GetArrayItem` _keys_5 _item_num_4))
      (`SceneComponent.K2_SetRelativeTransform` (`self.Item`) (`.Transform_122_52165CD641C2D4A94A776894C4A9C928` (break `/Game/Blueprints/Data/Struct/ItemInfo/Heat_Item_Info` (`|GetArrayItem` _values_5 _item_num_4))) false false))
    (:`NewEnumerator10`
      (bind _keys_6 (`BlueprintMapLibrary.Map_Keys` _distract_item))
      (bind _values_6 (`BlueprintMapLibrary.Map_Values` _distract_item))
      (`StaticMeshComponent.SetStaticMesh` (`self.Item`) (`|GetArrayItem` _keys_6 _item_num_3))
      (`SceneComponent.K2_SetRelativeTransform` (`self.Item`) (`.Transform_122_52165CD641C2D4A94A776894C4A9C928` (break `/Game/Blueprints/Data/Struct/ItemInfo/Distract_Item_Info` (`|GetArrayItem` _values_6 _item_num_3))) false false))))

(event `Set Current Item`
  ;[0 0 0] Setting Equipped Item to store into Current Item Type
  (switch `/Game/Blueprints/Data/Enum/ItemTypes/ItemType_Enum` (`self.Item Class`)
    (:`NewEnumerator7`
      (set `self.Current_Item` "NewEnumerator7")
      (`KismetArrayLibrary.Array_Set` (`self.Current_Items`) 0 (`StaticMeshComponent.StaticMesh` (`self.Item`))))
    (:`NewEnumerator11`
      (set `self.Current_Item` "NewEnumerator11")
      (`KismetArrayLibrary.Array_Set` (`self.Current_Items`) 1 (`StaticMeshComponent.StaticMesh` (`self.Item`))))
    (:`NewEnumerator12`
      (set `self.Current_Item` "NewEnumerator12")
      (`KismetArrayLibrary.Array_Set` (`self.Current_Items`) 2 (`StaticMeshComponent.StaticMesh` (`self.Item`))))
    (:`NewEnumerator14`
      (set `self.Current_Item` "NewEnumerator14")
      (`KismetArrayLibrary.Array_Set` (`self.Current_Items`) 3 (`StaticMeshComponent.StaticMesh` (`self.Item`))))
    (:`NewEnumerator0`
      (set `self.Current_Item` "NewEnumerator0")
      (`KismetArrayLibrary.Array_Set` (`self.Current_Items`) 4 (`StaticMeshComponent.StaticMesh` (`self.Item`))))
    (:`NewEnumerator15`
      (set `self.Current_Item` "NewEnumerator15")
      (`KismetArrayLibrary.Array_Set` (`self.Current_Items`) 5 (`StaticMeshComponent.StaticMesh` (`self.Item`))))
    (:`NewEnumerator10`
      (set `self.Current_Item` "NewEnumerator10")
      (`KismetArrayLibrary.Array_Set` (`self.Current_Items`) 6 (`StaticMeshComponent.StaticMesh` (`self.Item`))))))

(event `Swap Current Item`
  (bind _output (`|GetArrayItem` (`self.Current_Items`)))
  ;[0 0 0] Swapping Current Item
  (switch `/Game/Blueprints/Data/Enum/ItemTypes/ItemType_Current` (`self.Current_Item`)
    (:`NewEnumerator7`
      ;;[0 0 0] Setting Current Item to Health Item
      (`/Engine/EditorBlueprintResources/StandardMacros.IsValid` (`|GetArrayItem` (`self.Current_Items`) 1)
        (:`Is Valid`
          (bind _keys (`BlueprintMapLibrary.Map_Keys` (`self.Health Item`)))
          (set `self.Item Num` (`KismetArrayLibrary.Array_Find` _keys (`|GetArrayItem` (`self.Current_Items`) 1)))
          (bind _values (`BlueprintMapLibrary.Map_Values` (`self.Health Item`)))
          (bind (_itemclass _itemtype _transform) (break `/Game/Blueprints/Data/Struct/ItemInfo/Health_Item_Info` (`|GetArrayItem` _values (`self.Item Num`))))
          (set `self.Item Class` _itemclass)
          (`StaticMeshComponent.SetStaticMesh` (`self.Item`) (`|GetArrayItem` (`self.Current_Items`) 1))
          (`SceneComponent.K2_SetRelativeTransform` (`self.Item`) _transform false false)
          (set `self.Current_Item` "NewEnumerator11"))
        (:`Is Not Valid`
          ;;[0 0 0] Setting Current Item to Stamina Item
          (`/Engine/EditorBlueprintResources/StandardMacros.IsValid` (`|GetArrayItem` (`self.Current_Items`) 2) :!label _label
            (:`Is Valid`
              (bind _keys_2 (`BlueprintMapLibrary.Map_Keys` (`self.Stamina Item`)))
              (set `self.Item Num` (`KismetArrayLibrary.Array_Find` _keys_2 (`|GetArrayItem` (`self.Current_Items`) 2)))
              (bind _values_2 (`BlueprintMapLibrary.Map_Values` (`self.Stamina Item`)))
              (bind (_itemclass_2 _itemtype_2 _transform_2) (break `/Game/Blueprints/Data/Struct/ItemInfo/Stamina_Item_Info` (`|GetArrayItem` _values_2 (`self.Item Num`))))
              (set `self.Item Class` _itemclass_2)
              (`StaticMeshComponent.SetStaticMesh` (`self.Item`) (`|GetArrayItem` (`self.Current_Items`) 2))
              (`SceneComponent.K2_SetRelativeTransform` (`self.Item`) _transform_2 false false)
              (set `self.Current_Item` "NewEnumerator12"))
            (:`Is Not Valid`
              ;;[0 0 0] Setting Current Item to Infection Item
              (`/Engine/EditorBlueprintResources/StandardMacros.IsValid` (`|GetArrayItem` (`self.Current_Items`) 3) :!label _label_2
                (:`Is Valid`
                  (bind _keys_3 (`BlueprintMapLibrary.Map_Keys` (`self.Infection Item`)))
                  (set `self.Item Num` (`KismetArrayLibrary.Array_Find` _keys_3 (`|GetArrayItem` (`self.Current_Items`) 3)))
                  (bind _values_3 (`BlueprintMapLibrary.Map_Values` (`self.Infection Item`)))
                  (bind (_itemclass_3 _itemtype_3 _transform_3) (break `/Game/Blueprints/Data/Struct/ItemInfo/Infection_Item_Info` (`|GetArrayItem` _values_3 (`self.Item Num`))))
                  (set `self.Item Class` _itemclass_3)
                  (`StaticMeshComponent.SetStaticMesh` (`self.Item`) (`|GetArrayItem` (`self.Current_Items`) 3))
                  (`SceneComponent.K2_SetRelativeTransform` (`self.Item`) _transform_3 false false)
                  (set `self.Current_Item` "NewEnumerator14"))
                (:`Is Not Valid`
                  ;;[0 0 0] Setting Current Item to Explosive Item
                  (`/Engine/EditorBlueprintResources/StandardMacros.IsValid` (`|GetArrayItem` (`self.Current_Items`) 4) :!label _label_3
                    (:`Is Valid`
                      (bind _keys_4 (`BlueprintMapLibrary.Map_Keys` (`self.Explosive Item`)))
                      (set `self.Item Num` (`KismetArrayLibrary.Array_Find` _keys_4 (`|GetArrayItem` (`self.Current_Items`) 4)))
                      (bind _values_4 (`BlueprintMapLibrary.Map_Values` (`self.Explosive Item`)))
                      (bind (_itemclass_4 _itemtype_4 _transform_4) (break `/Game/Blueprints/Data/Struct/ItemInfo/Explosive_Item_Info` (`|GetArrayItem` _values_4 (`self.Item Num`))))
                      (set `self.Item Class` _itemclass_4)
                      (`StaticMeshComponent.SetStaticMesh` (`self.Item`) (`|GetArrayItem` (`self.Current_Items`) 4))
                      (`SceneComponent.K2_SetRelativeTransform` (`self.Item`) _transform_4 false false)
                      (set `self.Current_Item` "NewEnumerator0"))
                    (:`Is Not Valid`
                      ;;[0 0 0] Setting Current Item to Heat Item
                      (`/Engine/EditorBlueprintResources/StandardMacros.IsValid` (`|GetArrayItem` (`self.Current_Items`) 5) :!label _label_4
                        (:`Is Valid`
                          (bind _keys_5 (`BlueprintMapLibrary.Map_Keys` (`self.Heat Item`)))
                          (set `self.Item Num` (`KismetArrayLibrary.Array_Find` _keys_5 (`|GetArrayItem` (`self.Current_Items`) 5)))
                          (bind _values_5 (`BlueprintMapLibrary.Map_Values` (`self.Heat Item`)))
                          (bind (_itemclass_5 _itemtype_5 _transform_5) (break `/Game/Blueprints/Data/Struct/ItemInfo/Heat_Item_Info` (`|GetArrayItem` _values_5 (`self.Item Num`))))
                          (set `self.Item Class` _itemclass_5)
                          (`StaticMeshComponent.SetStaticMesh` (`self.Item`) (`|GetArrayItem` (`self.Current_Items`) 5))
                          (`SceneComponent.K2_SetRelativeTransform` (`self.Item`) _transform_5 false false)
                          (set `self.Current_Item` "NewEnumerator15"))
                        (:`Is Not Valid`
                          ;;[0 0 0] Setting Current Item to Distract Item
                          (`/Engine/EditorBlueprintResources/StandardMacros.IsValid` (`|GetArrayItem` (`self.Current_Items`) 6) :!label _label_5
                            (:`Is Valid`
                              (bind _keys_6 (`BlueprintMapLibrary.Map_Keys` (`self.Distract Item`)))
                              (set `self.Item Num` (`KismetArrayLibrary.Array_Find` _keys_6 (`|GetArrayItem` (`self.Current_Items`) 6)))
                              (bind _values_6 (`BlueprintMapLibrary.Map_Values` (`self.Distract Item`)))
                              (bind (_itemclass_6 _itemtype_6 _transform_6) (break `/Game/Blueprints/Data/Struct/ItemInfo/Distract_Item_Info` (`|GetArrayItem` _values_6 (`self.Item Num`))))
                              (set `self.Item Class` _itemclass_6)
                              (`StaticMeshComponent.SetStaticMesh` (`self.Item`) (`|GetArrayItem` (`self.Current_Items`) 6))
                              (`SceneComponent.K2_SetRelativeTransform` (`self.Item`) _transform_6 false false)
                              (set `self.Current_Item` "NewEnumerator10"))
                            (:`Is Not Valid`
                              ;;[0 0 0] Setting Current Item to No Item
                              (`/Engine/EditorBlueprintResources/StandardMacros.IsValid` _output :!label _label_6
                                (:`Is Not Valid`
                                  (`StaticMeshComponent.SetStaticMesh` (`self.Item`) _output)
                                  (set `self.Item Class` "NewEnumerator7")
                                  (set `self.Item Num` 0)
                                  (set `self.Current_Item` "NewEnumerator7"))))))))))))))))
    (:`NewEnumerator11`
      (goto _label))
    (:`NewEnumerator12`
      (goto _label_2))
    (:`NewEnumerator14`
      (goto _label_3))
    (:`NewEnumerator0`
      (goto _label_4))
    (:`NewEnumerator15`
      (goto _label_5))
    (:`NewEnumerator10`
      (goto _label_6))))