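; Actor component that tracks an infection level on its owning actor.
; On begin play it caches the owner; each Actor Infected event raises Infection by a fixed step, clamped to a percentage-style range.
; The new value is printed to screen as debug output, with no further effects in this graph.
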(event `self.ReceiveBeginPlay`
  ;[0 0 0] Event Begin Play
  (set `self.Infection` (`self.Infection`))
  (set `self.Owner` (`self.GetOwner`)))

(event `Actor Infected`
  ;[0 0 0] Actor Infected
  (bind _output_get (set `self.Infection` (`KismetMathLibrary.Clamp` (+ (`self.Infection`) 10) 0 100)))
  (`KismetSystemLibrary.PrintString` (`KismetStringLibrary.Conv_IntToString` _output_get)))