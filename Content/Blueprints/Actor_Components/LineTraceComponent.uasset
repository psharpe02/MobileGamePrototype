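; Actor component that gives its owner a weapon line trace and a distance-based target lock state.
; WeaponLineTrace multi-traces from a socket along the owner's forward vector, records new hits matching the Actors class list in TargetHit, and sets TargetedActor.
; It spawns an emitter and sound on new targets, non-matching class comparisons and misses.
; TargetActor sets TargetLock by TargetDistance, or toggles it when no target is valid.
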(event `self.ReceiveBeginPlay`
  ;[0 0 0] Event Begin Play
  (set `self.Owner` (`self.GetOwner`)))

(event `Weapon Line Trace`
  (params (Target :type "SceneComponent Object Reference") (InSocketName :type Name :default "Projectile") (`Line Trace Range` :type "Float (double-precision)" :default 0.0) (Sound :type "SoundBase Object Reference") (Emitter :type "ParticleSystem Object Reference"))
  (bind _owner (`self.Owner`))
  ;[0 0 0] Assign Weapon Line Trace to Actor
  (bind _output_get (set `self.Socket Location` (`SceneComponent.GetSocketLocation` Target InSocketName)))
  (bind (_outhits _returnvalue) (`KismetSystemLibrary.LineTraceMulti` _output_get (+ (`Actor.K2_GetActorLocation` _owner) (* (`Actor.GetActorForwardVector` _owner) `Line Trace Range`)) "TraceTypeQuery1" false (`|MakeArray` (`self.Owner`)) "ForDuration"))
  ;[0 0 0] For Each Loop Break Result
  (if _returnvalue
    (for _array_element _outhits
      ;[0 0 0] Checks if hit actor's class is assigned in an array
      (for _array_element_2 (`self.Actors`)
        (bind (_bblockinghit _binitialoverlap _time _distance _location _impactpoint _normal _impactnormal _physmat _hitactor) (`GameplayStatics.BreakHitResult` _array_element))
        (if (== _array_element_2 (`GameplayStatics.GetObjectClass` _hitactor))
          (`KismetSystemLibrary.PrintString` "Actors Hit")
          ;[0 0 0] Check If Enemy Was Already Hit
          (if (not (`KismetArrayLibrary.Array_Contains` (`self.TargetHit`) _hitactor))
            ;[0 0 0] Add To Hit Targets
            (`KismetArrayLibrary.Array_Add` (`self.TargetHit`) _hitactor)
            (set `self.Targeted Actor` _hitactor)
            ;[0 0 0] Spawns Emitter from Socket Location
            (`GameplayStatics.SpawnEmitterAtLocation` Emitter (`self.Socket Location`) (struct) (0.1 0.1 0.1) :!label _label)
            ;[0 0 0] lays Sound Effect at Owner's Location
            (`GameplayStatics.PlaySoundAtLocation` Sound (`Actor.K2_GetActorLocation` (`self.Owner`)) (struct) 1.0 1.0 0.0 null null null null))
          (else
            (`KismetSystemLibrary.PrintString` (`KismetSystemLibrary.GetDisplayName` _hitactor))
            (goto _label)))))
    (else
      (goto _label))))

(event `Target Actor`
  ;[0 0 0] Checks if hit actor is valid
  (`/Engine/EditorBlueprintResources/StandardMacros.IsValid` (`self.Targeted Actor`)
    (:`Is Valid`
      ;[0 0 0] Setting Target Lock Boolean based on Check
      (if (< (`KismetMathLibrary.VSize` (- (`Actor.K2_GetActorLocation` (`self.Targeted Actor`)) (`Actor.K2_GetActorLocation` (`self.Owner`)))) (`self.Target Distance`))
        (set `self.TargetLock` true)
        (else
          (set `self.TargetLock` false)
          (set `self.Targeted Actor` null))))
    (:`Is Not Valid`
      ;[0 0 0] Setting Target Lock Boolean if targeted actor is invalid
      (if (`self.TargetLock`)
        (set `self.TargetLock` false)
        (set `self.Targeted Actor` null)
        (else
          (set `self.TargetLock` true))))))