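; Cover actor that tells the player character's animation instance whether cover is available, based on overlap with its Box component.
; A Cover event stores the passed value in CanCover and forwards it through CoverMessage while the player overlaps the box.
; When an end overlap leaves the player outside the box, CanCover is cleared and sent the same way.
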(event `/Game/Blueprints/BP_Interaction.Cover`
  (params (Cover :type Boolean))
  (bind _returnvalue (`GameplayStatics.GetPlayerCharacter` 0))
  ;[0 0 0] Begin Overlapping with Cover
  (set `self.Can Cover` Cover)
  (if (`PrimitiveComponent.IsOverlappingActor` (`self.Box`) _returnvalue)
    (message `/Game/Blueprints/BP_Interaction.Cover` (`SkeletalMeshComponent.GetAnimInstance` (`Character.Mesh` _returnvalue)) (`self.Can Cover`))))

(event `self.Box.OnComponentEndOverlap`
  (params (OverlappedComponent :type "PrimitiveComponent Object Reference") (OtherActor :type "Actor Object Reference") (OtherComp :type "PrimitiveComponent Object Reference") (OtherBodyIndex :type Integer))
  (bind _returnvalue (`GameplayStatics.GetPlayerCharacter` 0))
  ;[0 0 0] End Overlapping with Cover
  (if (not (`PrimitiveComponent.IsOverlappingActor` (`self.Box`) _returnvalue))
    (bind _output_get (set `self.Can Cover` false))
    (message `/Game/Blueprints/BP_Interaction.Cover` (`SkeletalMeshComponent.GetAnimInstance` (`Character.Mesh` _returnvalue)) _output_get)))

(fn `UserConstructionScript`)