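; Weapon pickup actor that hands its configured weapon to the player on overlap.
; The construction script picks the mesh from per-class map keys using the WeaponClass enum and WeaponNum index, offsetting melee meshes by their WeaponSocket location.
; When the player character enters the box, it disables input and stops rotating.
; After a delay, it sends EquipWeaponMessage with mesh, class and index, restores input and destroys itself.
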(event `self.Box.OnComponentBeginOverlap`
  (params (OverlappedComponent :type "PrimitiveComponent Object Reference") (OtherActor :type "Actor Object Reference") (OtherComp :type "PrimitiveComponent Object Reference") (OtherBodyIndex :type Integer) (bFromSweep :type Boolean) (SweepResult :type "HitResult Structure (by ref)"))
  (bind _returnvalue (`GameplayStatics.GetPlayerController` 0))
  (bind _returnvalue_2 (`GameplayStatics.GetPlayerController` 0))
  (if (== OtherActor (`GameplayStatics.GetPlayerCharacter` 0))
    (`self.DisableInput` _returnvalue _returnvalue)
    (set `RotatingMovementComponent.RotationRate` (struct) (`self.RotatingMovement`))
    (`KismetSystemLibrary.Delay` 3.0)
    (message `/Game/Blueprints/BP_Weapon.Equip Weapon` (`GameplayStatics.GetPlayerCharacter` 0) (`self.Weapon`) (`self.Weapon Class`) (`self.WeaponNum`))
    (`self.EnableInput` _returnvalue_2 _returnvalue_2)
    (`self.K2_DestroyActor`)))

(fn `UserConstructionScript`
  ;[0 0 0] Weapon Classes with using Map and Enums to set specific Weapons publicly
  (switch `/Game/Blueprints/Data/Enum/WeaponType_Enum` (`self.Weapon Class`)
    (:`NewEnumerator7`
      (`StaticMeshComponent.SetStaticMesh` (`self.Weapon`) null))
    (:`NewEnumerator0`
      (bind _keys (`BlueprintMapLibrary.Map_Keys` (`self.Melee Weapon`)))
      (bind _output (`|GetArrayItem` _keys (`self.WeaponNum`)))
      (`StaticMeshComponent.SetStaticMesh` (`self.Weapon`) _output)
      (`SceneComponent.K2_SetRelativeLocation` (`self.Weapon`) (`StaticMeshSocket.RelativeLocation` (`StaticMesh.FindSocket` _output "WeaponSocket")) false false))
    (:`NewEnumerator1`
      (bind _keys_2 (`BlueprintMapLibrary.Map_Keys` (`self.Pistol Weapon`)))
      (`StaticMeshComponent.SetStaticMesh` (`self.Weapon`) (`|GetArrayItem` _keys_2 (`self.WeaponNum`))))
    (:`NewEnumerator2`
      (bind _keys_3 (`BlueprintMapLibrary.Map_Keys` (`self.SMG Weapon`)))
      (`StaticMeshComponent.SetStaticMesh` (`self.Weapon`) (`|GetArrayItem` _keys_3 (`self.WeaponNum`))))
    (:`NewEnumerator5`
      (bind _keys_4 (`BlueprintMapLibrary.Map_Keys` (`self.AR Weapon`)))
      (`StaticMeshComponent.SetStaticMesh` (`self.Weapon`) (`|GetArrayItem` _keys_4 (`self.WeaponNum`))))
    (:`NewEnumerator4`
      (bind _keys_5 (`BlueprintMapLibrary.Map_Keys` (`self.Shotgun Weapon`)))
      (`StaticMeshComponent.SetStaticMesh` (`self.Weapon`) (`|GetArrayItem` _keys_5 (`self.WeaponNum`))))
    (:`NewEnumerator3`
      (bind _keys_6 (`BlueprintMapLibrary.Map_Keys` (`self.RL Weapon`)))
      (`StaticMeshComponent.SetStaticMesh` (`self.Weapon`) (`|GetArrayItem` _keys_6 (`self.WeaponNum`))))
    (:`NewEnumerator8`
      (bind _keys_7 (`BlueprintMapLibrary.Map_Keys` (`self.SR Weapon`)))
      (`StaticMeshComponent.SetStaticMesh` (`self.Weapon`) (`|GetArrayItem` _keys_7 (`self.WeaponNum`))))))