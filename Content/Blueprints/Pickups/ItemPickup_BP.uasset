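; Item pickup actor that rotates in the level and equips its item on the player when they overlap its box.
; The construction script copies the item class and number into the item component and calls its SelectItem with the chosen item.
; On player overlap it disables input and stops the rotation, waits briefly, sends EquipItemMessage to the character, then restores input and destroys itself.
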(event `self.Box.OnComponentBeginOverlap`
  (params (OverlappedComponent :type "PrimitiveComponent Object Reference") (OtherActor :type "Actor Object Reference") (OtherComp :type "PrimitiveComponent Object Reference") (OtherBodyIndex :type Integer) (bFromSweep :type Boolean) (SweepResult :type "HitResult Structure (by ref)"))
  (bind _returnvalue (`GameplayStatics.GetPlayerController` 0))
  (bind _returnvalue_2 (`GameplayStatics.GetPlayerController` 0))
  (if (== OtherActor (`GameplayStatics.GetPlayerCharacter` 0))
    (`self.DisableInput` _returnvalue _returnvalue)
    (set `RotatingMovementComponent.RotationRate` (struct) (`self.RotatingMovement`))
    (`KismetSystemLibrary.Delay` 3.0)
    (message `/Game/Blueprints/BP_Pickup.Equip Item` (`GameplayStatics.GetPlayerCharacter` 0) (`self.Item Class`) (`self.Item Num`))
    (`self.EnableInput` _returnvalue_2 _returnvalue_2)
    (`self.K2_DestroyActor`)))

(fn `UserConstructionScript`
  ;[0 0 0] Setting Item Class and Num from Select Item Event
  (set `/Game/Blueprints/Actor_Components/ItemComponent.Item Class` (`self.Item Class`) (`self.ItemComponent`))
  (set `/Game/Blueprints/Actor_Components/ItemComponent.Item Num` (`self.Item Num`) (`self.ItemComponent`))
  (`/Game/Blueprints/Actor_Components/ItemComponent.Select Item` (`self.ItemComponent`) (`self.Item`)))